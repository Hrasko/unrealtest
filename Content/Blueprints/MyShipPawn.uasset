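; MyShipPawn is a ship pawn that fires projectiles and creates its ShipHUD widget on begin play.
; Holding fire shoots immediately, then repeats on a looping timer set by RoundsPerSecond until release clears it and resets the DoOnce.
; Each shot spawns a projectile at FiringPoint with damage scaled by current Power, then drains Power.
; Tick regenerates clamped Power and prints the ship's location, only on the authority.
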(event `self.ReceiveBeginPlay`
  (bind _returnvalue (`|CreateWidget` "/Game/Blueprints/ShipHUD.ShipHUD_C"))
  (`UserWidget.AddToViewport` _returnvalue 0))

(event `self.FirePressed`
  (`/Engine/EditorBlueprintResources/StandardMacros.DoOnce` false :!label _label
    (:`Completed`
      (`self.Fire`)
      (bind _returnvalue (`KismetSystemLibrary.K2_SetTimer` null "Fire" (/ 1.0 (`self.Rounds per Second`)) true)))))

(event `self.ReceiveActorBeginOverlap`
  (params (OtherActor :type "Actor Object Reference")))

(event `self.FireReleased`
  (`KismetSystemLibrary.K2_ClearTimerHandle` null (stale `self.FirePressed` _returnvalue))
  (goto _label :!via `Reset`))

(event `self.ReceiveTick`
  (params (DeltaSeconds :type "Float (single-precision)"))
  (`/Engine/EditorBlueprintResources/ActorMacros.Switch Has Authority`
    (:`Authority`
      (`KismetSystemLibrary.PrintString` (`KismetStringLibrary.Conv_VectorToString` (`self.K2_GetActorLocation`)))
      (set `self.Power` (`KismetMathLibrary.FClamp` (+ (* DeltaSeconds (`self.Power Recover`)) (`self.Power`)) (`self.GetMinPower`) (`self.GetMaxPower`))))))

(event `Fire`
  (bind _power (`self.Power`))
  (bind _returnvalue (`|SpawnActorFromClass` "/Game/Blueprints/Projectile.Projectile_C" (`SceneComponent.K2_GetComponentToWorld` (`self.FiringPoint`)) "Undefined" "OverrideRootScale"))
  (message `/Game/Blueprints/IDamager.SetDamageValue` _returnvalue (* _power 5.0))
  (set `self.Power` (`KismetMathLibrary.FClamp` (- _power (`self.Power Decay`)) (`self.GetMinPower`) (`self.GetMaxPower`))))

(fn `UserConstructionScript`)