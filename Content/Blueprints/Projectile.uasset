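; Projectile actor that deals damage to non-player actors it overlaps and then destroys itself.
; On overlap, it skips actors tagged Player, only printing a debug string for them.
; Other actors implementing the IDamageble interface receive the stored Damage through AffectHealthMessage, and the projectile is destroyed whether or not they implement it.
; A SetDamageValue event sets the damage amount from outside.
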(event `self.ReceiveBeginPlay`)

(event `self.ReceiveActorBeginOverlap`
  (params (OtherActor :type "Actor Object Reference"))
  (if (not (`self.ActorHasTag` OtherActor "Player"))
    (if (`KismetSystemLibrary.DoesImplementInterface` OtherActor "/Game/Blueprints/IDamageble.IDamageble_C")
      (message `/Game/Blueprints/IDamageble.AffectHealth` OtherActor (`self.Damage`)))
    (`self.K2_DestroyActor`)
    (else
      (`KismetSystemLibrary.PrintString` "True"))))

(event `self.ReceiveTick`
  (params (DeltaSeconds :type "Float (single-precision)")))

(event `/Game/Blueprints/IDamager.SetDamageValue`
  (params (Damage :type "Float (single-precision)"))
  (set `self.Damage` Damage))

(fn `UserConstructionScript`)