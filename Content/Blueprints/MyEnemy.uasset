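; MyEnemy is an enemy Blueprint that handles health changes and an electric special-hit effect.
; AffectHealth forwards its delta to TakeDamage.
; TakeSpecial attaches an electricity arc to the enemy mesh and re-aims the beam at the player pawn every 0.2 seconds through a looping Delay.
; A parallel Delay destroys the arc after three seconds, but the re-aim loop has no exit.
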(event `self.ReceiveBeginPlay`)

(event `/Game/Blueprints/IDamageble.AffectHealth`
  (params (Delta :type "Float (single-precision)"))
  (`self.TakeDamage` Delta))

(event `self.ReceiveActorBeginOverlap`
  (params (OtherActor :type "Actor Object Reference")))

(event `self.TakeSpecial`
  (bind _returnvalue (`GameplayStatics.SpawnEmitterAttached` "/Game/ExampleContent/Effects/ParticleSystems/P_electricity_arc.P_electricity_arc" (`self.EnemyMesh`) "None" (0.0 0.0 0.0) (struct) "SnapToTargetIncludingScale"))
  (`ParticleSystemComponent.SetBeamTargetPoint` _returnvalue 0 (`self.K2_GetActorLocation` (`GameplayStatics.GetPlayerPawn` 0)) 0 :!label _label)
  (`|ExecutionSequence`
    (:`then_0`
      (`KismetSystemLibrary.Delay` 3.0)
      (`ActorComponent.K2_DestroyComponent` _returnvalue))
    (:`then_1`
      (`KismetSystemLibrary.Delay` 0.2)
      (goto _label))))

(event `self.ReceiveTick`
  (params (DeltaSeconds :type "Float (single-precision)")))

(fn `UserConstructionScript`)